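; Laser puzzle box that lights its core while a laser line touches it and supplies a redirected beam path.
; Core overlaps with BP_LaserLine apply the stored material on begin and restore the deactivated laser material on end.
; Reflect returns start and end points along the Arrow's forward vector, using a maximum distance.
; The IsActorActivated interface function always returns false.
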(event OnComponentBeginOverlap(Core)
  (params (OverlappedComponent :type Primitive%20Component%20Object%20Reference) (OtherActor :type Actor%20Object%20Reference) (OtherComp :type Primitive%20Component%20Object%20Reference) (OtherBodyIndex :type Integer) (bFromSweep :type Boolean) (SweepResult :type Hit%20Result%20Structure%20%28by%20ref%29))
  ;[1 1 1] Trigger core change
  (if (== (Utilities|GetClass OtherActor) "/Game/PuzzleLasers/BluePrints/Actos/Laser/BP_LaserLine.BP_LaserLine_C")
    (CallFunction|ChangeCore (Variables|PuzzleLaserKit|GetMaterial))))

(event OnComponentEndOverlap(Core)
  (params (OverlappedComponent :type Primitive%20Component%20Object%20Reference) (OtherActor :type Actor%20Object%20Reference) (OtherComp :type Primitive%20Component%20Object%20Reference) (OtherBodyIndex :type Integer))
  ;[1 1 1] Trigger core change
  (if (== (Utilities|GetClass OtherActor) "/Game/PuzzleLasers/BluePrints/Actos/Laser/BP_LaserLine.BP_LaserLine_C")
    (CallFunction|Resetcore)))

(event Custom|change%20core
  (params (Material :type Material%20Interface%20Object%20Reference))
  ;[1 1 1] Change Core Instance
  (bind _output_get (Variables|PuzzleLaserKit|SetMaterial Material))
  (Rendering|Material|SetMaterial (Variables|Default|GetCore) 0 _output_get))

(event Custom|resetcore
  ;[1 1 1] Change Core Instance
  (Rendering|Material|SetMaterial (Variables|Default|GetCore) 0 "/Game/PuzzleLasers/Materials/Lasers/M_laser_Deactivated.M_laser_Deactivated"))

(fn ConstructionScript)

(fn Reflect
  (bind _arrow (Variables|Default|GetArrow))
  (bind _returnvalue (Transformation|GetWorldLocation _arrow))
  ;[1 1 1] Reflect in direction of arrow
  (return _returnvalue (+ _returnvalue (* (Math|Vector|GetForwardVector _arrow) (Variables|PuzzleLaserKit|GetMaxNonReflectDistantion)))))

(fn IsActorActivatedBPI
  (return false))