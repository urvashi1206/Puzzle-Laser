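; Puzzle door with four locks that slides open in four panels when the player overlaps its box and closes when they leave.
; Interface-style events set an On/Off selection that each DoorUnlock event uses to clear or set its lock, with material and sound feedback.
; Opening first checks that all locks are clear, setting an unlocked flag that is never reset here.
; A looping timer spins the first two lock orbs.
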(event OnComponentBeginOverlap(Box)
  (params (OverlappedComponent :type Primitive%20Component%20Object%20Reference) (OtherActor :type Actor%20Object%20Reference) (OtherComp :type Primitive%20Component%20Object%20Reference) (OtherBodyIndex :type Integer) (bFromSweep :type Boolean) (SweepResult :type Hit%20Result%20Structure%20%28by%20ref%29))
  ;[1 1 1] Open Door on overlap with player
  (if (Actor|ActorHasTag OtherActor "Player")
    (CallFunction|OpenBPI)))

(event OnComponentEndOverlap(Box)
  (params (OverlappedComponent :type Primitive%20Component%20Object%20Reference) (OtherActor :type Actor%20Object%20Reference) (OtherComp :type Primitive%20Component%20Object%20Reference) (OtherBodyIndex :type Integer))
  ;[1 1 1] Open Door on overlap with player
  (if (Actor|ActorHasTag OtherActor "Player")
    (CallFunction|CloseBPI)))

(event Custom|rotate
  ;[1 0.1165 0.8849] Set rotation of the lock orbs on door
  (bind _spheres (Timeline|Timeline_1 PlayFromStart)
    (:Update
      (Transformation|SetRelativeRotation (Variables|Default|GetLockOne) (Math|Rotator|MakeRotator 0.0 0.0 _spheres) false false)
      (Transformation|SetRelativeRotation (Variables|Default|GetLockTwo) (Math|Rotator|MakeRotator 0.0 0.0 _spheres) false false))))

(event Custom|Check%20Locks
  ;[1 0.8818 0] Check if all locks have been unlocked
  (if (not (Variables|DoorLocks|GetLockOne?))
    (if (not (Variables|DoorLocks|GetLockTwo?))
      (if (not (Variables|DoorLocks|GetLockThree?))
        (if (not (Variables|DoorLocks|GetLockFour?))
          (Variables|DoorDefaults|SetDoorUnlocked true))))))

(event EventDoorUnlockThree
  ;[1 0.1352 0.265] Set Door Locks
  (switch Utilities|FlowControl|Switch|SwitchonE_On_Off (Variables|DoorDefaults|GetSelection)
    (:NewEnumerator0
      (Audio|PlaySoundatLocation "/Game/PuzzleLasers/sounds/SW_Activate.SW_Activate" (Transformation|GetActorLocation) "0, 0, 0" 1.0 1.0 0.0 0 0 0 0)
      (Rendering|Material|SetMaterial (Variables|Default|GetLockThree) 0 0)
      (Variables|DoorLocks|SetLockThree? false))
    (:NewEnumerator1
      (Rendering|Material|SetMaterial (Variables|Default|GetLockThree) 0 0)
      (Variables|DoorLocks|SetLockThree? true))))

(event EventDoorUnlockFour
  ;[1 0.1352 0.265] Set Door Locks
  (switch Utilities|FlowControl|Switch|SwitchonE_On_Off (Variables|DoorDefaults|GetSelection)
    (:NewEnumerator0
      (Audio|PlaySoundatLocation "/Game/PuzzleLasers/sounds/SW_Activate.SW_Activate" (Transformation|GetActorLocation) "0, 0, 0" 1.0 1.0 0.0 0 0 0 0)
      (Rendering|Material|SetMaterial (Variables|Default|Get%20LockFour) 0 0)
      (Variables|DoorLocks|SetLockFour? false))
    (:NewEnumerator1
      (Rendering|Material|SetMaterial (Variables|Default|Get%20LockFour) 0 0)
      (Variables|DoorLocks|SetLockFour? true))))

(event EventCloseBPI
  ;[1 0.2911 0.0904] Open / Close function call from interface
  (if (Variables|DoorDefaults|GetOpened?)
    (Variables|DoorDefaults|SetOpened? false)
    (Audio|PlaySoundatLocation "/Game/PuzzleLasers/sounds/SW_DoorClose.SW_DoorClose" (Transformation|GetActorLocation) "0, 0, 0" 1.0 1.0 0.0 0 0 0 0)
    (bind (_direction _top _zbottom _left1 _right1) (Timeline|Timeline_0 Reverse)
      (:Update
        (Transformation|SetRelativeLocation (Variables|Default|GetDoorTop) (Math|Vector|MakeVector 0.0 0.0 _top) false false)
        (Transformation|SetRelativeLocation (Variables|Default|GetDoorBottom) (Math|Vector|MakeVector 0.0 0.0 _zbottom) false false)
        (Transformation|SetRelativeLocation (Variables|Default|GetDoorLeft) (Math|Vector|MakeVector _left1 0.0 0.0) false false)
        (Transformation|SetRelativeLocation (Variables|Default|GetDoorRight) (Math|Vector|MakeVector _right1 0.0 0.0) false false)))))

(event EventOpenBPI
  ;[1 0.2911 0.0904] Open / Close function call from interface
  (CallFunction|CheckLocks)
  (if (Variables|DoorDefaults|GetDoorUnlocked)
    (if (not (Variables|DoorDefaults|GetOpened?))
      (Variables|DoorDefaults|SetOpened? true)
      (Audio|PlaySoundatLocation "/Game/PuzzleLasers/sounds/SW_DoorOpen.SW_DoorOpen" (Transformation|GetActorLocation) "0, 0, 0" 1.0 1.0 0.0 0 0 0 0)
      (bind (_direction _top _zbottom _left1 _right1) (Timeline|Timeline_0 Play)
        (:Update
          (Transformation|SetRelativeLocation (Variables|Default|GetDoorTop) (Math|Vector|MakeVector 0.0 0.0 _top) false false)
          (Transformation|SetRelativeLocation (Variables|Default|GetDoorBottom) (Math|Vector|MakeVector 0.0 0.0 _zbottom) false false)
          (Transformation|SetRelativeLocation (Variables|Default|GetDoorLeft) (Math|Vector|MakeVector _left1 0.0 0.0) false false)
          (Transformation|SetRelativeLocation (Variables|Default|GetDoorRight) (Math|Vector|MakeVector _right1 0.0 0.0) false false))))))

(event EventDoorUnlockOne
  ;[1 0.1352 0.265] Set Door Locks
  (switch Utilities|FlowControl|Switch|SwitchonE_On_Off (Variables|DoorDefaults|GetSelection)
    (:NewEnumerator0
      (Audio|PlaySoundatLocation "/Game/PuzzleLasers/sounds/SW_Activate.SW_Activate" (Transformation|GetActorLocation) "0, 0, 0" 1.0 1.0 0.0 0 0 0 0)
      (Rendering|Material|SetMaterial (Variables|Default|GetLockOne) 0 "/Game/PuzzleLasers/Materials/emissive/M_Activated.M_Activated")
      (Variables|DoorLocks|SetLockOne? false))
    (:NewEnumerator1
      (Rendering|Material|SetMaterial (Variables|Default|GetLockOne) 0 0)
      (Variables|DoorLocks|SetLockOne? true))))

(event EventBeginPlay
  ;[1 0.1165 0.8849] Set rotation of the lock orbs on door
  (Utilities|Time|SetTimerbyEvent (delegate Custom|rotate) 1.0 true))

(event EventOn
  ;[0.3445 1 0.0904] Turn Door on or off set in trigger
  (Variables|DoorDefaults|SetSelection "NewEnumerator0"))

(event EventOff
  ;[0.3445 1 0.0904] Turn Door on or off set in trigger
  (Variables|DoorDefaults|SetSelection "NewEnumerator1"))

(event EventDoorUnlockTwo
  ;[1 0.1352 0.265] Set Door Locks
  (switch Utilities|FlowControl|Switch|SwitchonE_On_Off (Variables|DoorDefaults|GetSelection)
    (:NewEnumerator0
      (Audio|PlaySoundatLocation "/Game/PuzzleLasers/sounds/SW_Activate.SW_Activate" (Transformation|GetActorLocation) "0, 0, 0" 1.0 1.0 0.0 0 0 0 0)
      (Rendering|Material|SetMaterial (Variables|Default|GetLockTwo) 0 0)
      (Variables|DoorLocks|SetLockTwo? false))
    (:NewEnumerator1
      (Rendering|Material|SetMaterial (Variables|Default|GetLockTwo) 0 0)
      (Variables|DoorLocks|SetLockTwo? true))))

(fn ConstructionScript
  (bind _lockone (Variables|Default|GetLockOne))
  (bind _lockthree (Variables|Default|GetLockThree))
  (bind __lockfour (Variables|Default|Get%20LockFour))
  (bind _locktwo (Variables|Default|GetLockTwo))
  ;[1 0.2834 0.9697] Change Lock material
  (Utilities|FlowControl|Sequence
    (:then_0
      (if (Variables|DoorLocks|GetLockOne?)
        (Rendering|Material|SetMaterial _lockone 0 "/Game/PuzzleLasers/demo/FirstPerson/Meshes/BaseMaterial.BaseMaterial")
        (else
          (Rendering|Material|SetMaterial _lockone 0 "/Game/PuzzleLasers/Materials/emissive/M_Activated.M_Activated"))))
    (:then_1
      (if (Variables|DoorLocks|GetLockTwo?)
        (Rendering|Material|SetMaterial _locktwo 0 "/Game/PuzzleLasers/demo/FirstPerson/Meshes/BaseMaterial.BaseMaterial")
        (else
          (Rendering|Material|SetMaterial _locktwo 0 "/Game/PuzzleLasers/Materials/emissive/M_Activated.M_Activated"))))
    (:then_2
      (if (Variables|DoorLocks|GetLockThree?)
        (Rendering|Material|SetMaterial _lockthree 0 0)
        (else
          (Rendering|Material|SetMaterial _lockthree 0 "/Game/PuzzleLasers/Materials/emissive/M_Activated.M_Activated"))))
    (:then_3
      (if (Variables|DoorLocks|GetLockFour?)
        (Rendering|Material|SetMaterial __lockfour 0 0)
        (else
          (Rendering|Material|SetMaterial __lockfour 0 "/Game/PuzzleLasers/Materials/emissive/M_Activated.M_Activated"))))))

(fn IsActorActivatedBPI
  (return false))